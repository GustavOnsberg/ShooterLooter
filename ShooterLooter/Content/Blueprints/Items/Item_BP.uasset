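; Base item actor that players can target for interaction or, if flagged, collect automatically.
; On an interaction check it hands its InteractionStuff and itself to the player as the crosshair interactable.
; Auto-pickup disables the box's collision and physics, then a looping timer eases the item toward the player before it is picked up and destroyed.
; The space check and pickup functions are empty stubs here.
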(event EventBeginPlay)

(event EventActorBeginOverlap
  (params (OtherActor :type Actor%20Object%20Reference)))

(event EventTick
  (params (DeltaSeconds :type Float%20%28single-precision%29)))

(event Custom|MoveTowardsPlayer
  (bind _player (Variables|Default|GetPlayer))
  (bind _returnvalue (Transformation|GetActorLocation _player))
  (Variables|Default|SetPickupMoveProgress (+ (Variables|Default|GetPickupMoveProgress) 0.02))
  (Transformation|SetActorLocation (Math|Interpolation|Ease "EaseIn" (Variables|Default|GetPickupMoveProgress) (Variables|Default|GetStartPickupLocation) (Math|Vector|MakeVector (.x _returnvalue) (.y _returnvalue) (+ (.z _returnvalue) 2e+01)) 2.0) false false))

(event EventTryAutomaticallyPickUp
  (params (Player :type Player%20Character%20BP%20Object%20Reference))
  (Variables|Default|SetPlayer Player)
  (if (.automaticallypickup (Variables|Default|GetInteractionStuff))
    (CallFunction|CheckifPlayerHaveSpace)
    (if (Variables|Default|GetPlayerHaveSpace)
      (Variables|Default|SetStartPickupLocation (Transformation|GetActorLocation))
      (CallFunction|StartPending)
      (Utilities|Time|SetTimerbyEvent (delegate Custom|MoveTowardsPlayer) 0.01 true)
      (Utilities|FlowControl|Delay 0.5)
      (CallFunction|PickUp (Variables|Default|GetPlayer))
      (Actor|DestroyActor))))

(event EventCheckInteraction
  (params (Player :type Player%20Character%20BP%20Object%20Reference))
  (Variables|/Game/Blueprints/PlayerCharacter_BP.PlayerCharacter_BP_C|SetInteractionStuff Player (Variables|Default|GetInteractionStuff))
  (Variables|/Game/Blueprints/PlayerCharacter_BP.PlayerCharacter_BP_C|SetIntractableInCrosshair Player self))

(fn ConstructionScript)

(fn StartPending
  (bind _box (Variables|Default|GetBox))
  (Collision|SetCollisionEnabled _box "NoCollision")
  (Physics|SetSimulatePhysics _box false))

(fn CheckifPlayerHaveSpace)

(fn PickUp
  (params (Player :type Player%20Character%20BP%20Object%20Reference)))