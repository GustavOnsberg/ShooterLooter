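; Ammo pickup that refills one of the player's six weapon ammo pools, chosen by its AmmoType.
; CheckifPlayerHaveSpace clears PlayerHaveSpace when that pool is at its maximum.
; StartPending adds Ammo to the player's pending count for that type.
; PickUp adds both Ammo and the pending count to the pool, deducts Ammo from pending, then clamps the pool to its maximum.
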(event EventBeginPlay)

(event EventActorBeginOverlap
  (params (OtherActor :type Actor%20Object%20Reference)))

(event EventTick
  (params (DeltaSeconds :type Float%20%28single-precision%29)))

(event EventCheckifPlayerHaveSpace
  (bind _player (Variables|Default|GetPlayer))
  (switch Utilities|FlowControl|Switch|SwitchonWeaponTypes (Variables|Default|GetAmmoType)
    (:NewEnumerator0
      (if (not (< (Variables|/Game/Blueprints/PlayerCharacter_BP.PlayerCharacter_BP_C|GetPistolAmmo _player) (Variables|/Game/Blueprints/PlayerCharacter_BP.PlayerCharacter_BP_C|GetMaxPistolAmmo _player)))
        (Variables|Default|SetPlayerHaveSpace false :!label _label)))
    (:NewEnumerator1
      (if (not (< (Variables|/Game/Blueprints/PlayerCharacter_BP.PlayerCharacter_BP_C|GetAssaultRifleAmmo _player) (Variables|/Game/Blueprints/PlayerCharacter_BP.PlayerCharacter_BP_C|GetMaxAssaultRifleAmmo _player)))
        (goto _label)))
    (:NewEnumerator2
      (if (not (< (Variables|/Game/Blueprints/PlayerCharacter_BP.PlayerCharacter_BP_C|GetSMGAmmo _player) (Variables|/Game/Blueprints/PlayerCharacter_BP.PlayerCharacter_BP_C|GetMaxSMGAmmo _player)))
        (goto _label)))
    (:NewEnumerator3
      (if (not (< (Variables|/Game/Blueprints/PlayerCharacter_BP.PlayerCharacter_BP_C|GetShotgunAmmo _player) (Variables|/Game/Blueprints/PlayerCharacter_BP.PlayerCharacter_BP_C|GetMaxShotgunAmmo _player)))
        (goto _label)))
    (:NewEnumerator4
      (if (not (< (Variables|/Game/Blueprints/PlayerCharacter_BP.PlayerCharacter_BP_C|GetSniperRifleAmmo _player) (Variables|/Game/Blueprints/PlayerCharacter_BP.PlayerCharacter_BP_C|GetMaxSniperRifleAmmo _player)))
        (goto _label)))
    (:NewEnumerator5
      (if (not (< (Variables|/Game/Blueprints/PlayerCharacter_BP.PlayerCharacter_BP_C|GetRocketLauncherAmmo _player) (Variables|/Game/Blueprints/PlayerCharacter_BP.PlayerCharacter_BP_C|GetMaxRocketLauncherAmmo _player)))
        (goto _label)))))

(event EventPickUp
  (params (Player :type Player%20Character%20BP%20Object%20Reference))
  (bind _ammo (Variables|Default|GetAmmo))
  (bind _ammo_2 (Variables|Default|GetAmmo))
  (switch Utilities|FlowControl|Switch|SwitchonWeaponTypes (Variables|Default|GetAmmoType)
    (:NewEnumerator0
      (Variables|/Game/Blueprints/PlayerCharacter_BP.PlayerCharacter_BP_C|SetPistolAmmo (Variables|Default|GetPlayer) (+ (Variables|/Game/Blueprints/PlayerCharacter_BP.PlayerCharacter_BP_C|GetPistolAmmo (Variables|Default|GetPlayer)) _ammo_2 (Variables|/Game/Blueprints/PlayerCharacter_BP.PlayerCharacter_BP_C|GetPendingPistolAmmo (Variables|Default|GetPlayer))))
      (Variables|/Game/Blueprints/PlayerCharacter_BP.PlayerCharacter_BP_C|SetPendingPistolAmmo (Variables|Default|GetPlayer) (- (Variables|/Game/Blueprints/PlayerCharacter_BP.PlayerCharacter_BP_C|GetPendingPistolAmmo (Variables|Default|GetPlayer)) _ammo))
      (if (> (Variables|/Game/Blueprints/PlayerCharacter_BP.PlayerCharacter_BP_C|GetPistolAmmo (Variables|Default|GetPlayer)) (Variables|/Game/Blueprints/PlayerCharacter_BP.PlayerCharacter_BP_C|GetMaxPistolAmmo (Variables|Default|GetPlayer)))
        (Variables|/Game/Blueprints/PlayerCharacter_BP.PlayerCharacter_BP_C|SetPistolAmmo (Variables|Default|GetPlayer) (Variables|/Game/Blueprints/PlayerCharacter_BP.PlayerCharacter_BP_C|GetMaxPistolAmmo (Variables|Default|GetPlayer)))))
    (:NewEnumerator1
      (Variables|/Game/Blueprints/PlayerCharacter_BP.PlayerCharacter_BP_C|SetAssaultRifleAmmo (Variables|Default|GetPlayer) (+ (Variables|/Game/Blueprints/PlayerCharacter_BP.PlayerCharacter_BP_C|GetAssaultRifleAmmo (Variables|Default|GetPlayer)) _ammo_2 (Variables|/Game/Blueprints/PlayerCharacter_BP.PlayerCharacter_BP_C|GetPendingAssaultRifleAmmo (Variables|Default|GetPlayer))))
      (Variables|/Game/Blueprints/PlayerCharacter_BP.PlayerCharacter_BP_C|SetPendingAssaultRifleAmmo (Variables|Default|GetPlayer) (- (Variables|/Game/Blueprints/PlayerCharacter_BP.PlayerCharacter_BP_C|GetPendingAssaultRifleAmmo (Variables|Default|GetPlayer)) _ammo))
      (if (> (Variables|/Game/Blueprints/PlayerCharacter_BP.PlayerCharacter_BP_C|GetAssaultRifleAmmo (Variables|Default|GetPlayer)) (Variables|/Game/Blueprints/PlayerCharacter_BP.PlayerCharacter_BP_C|GetMaxAssaultRifleAmmo (Variables|Default|GetPlayer)))
        (Variables|/Game/Blueprints/PlayerCharacter_BP.PlayerCharacter_BP_C|SetAssaultRifleAmmo (Variables|Default|GetPlayer) (Variables|/Game/Blueprints/PlayerCharacter_BP.PlayerCharacter_BP_C|GetMaxAssaultRifleAmmo (Variables|Default|GetPlayer)))))
    (:NewEnumerator2
      (Variables|/Game/Blueprints/PlayerCharacter_BP.PlayerCharacter_BP_C|SetSMGAmmo (Variables|Default|GetPlayer) (+ (Variables|/Game/Blueprints/PlayerCharacter_BP.PlayerCharacter_BP_C|GetSMGAmmo (Variables|Default|GetPlayer)) _ammo_2 (Variables|/Game/Blueprints/PlayerCharacter_BP.PlayerCharacter_BP_C|GetPendingSMGAmmo (Variables|Default|GetPlayer))))
      (Variables|/Game/Blueprints/PlayerCharacter_BP.PlayerCharacter_BP_C|SetPendingSMGAmmo (Variables|Default|GetPlayer) (- (Variables|/Game/Blueprints/PlayerCharacter_BP.PlayerCharacter_BP_C|GetPendingSMGAmmo (Variables|Default|GetPlayer)) _ammo))
      (if (> (Variables|/Game/Blueprints/PlayerCharacter_BP.PlayerCharacter_BP_C|GetSMGAmmo (Variables|Default|GetPlayer)) (Variables|/Game/Blueprints/PlayerCharacter_BP.PlayerCharacter_BP_C|GetMaxSMGAmmo (Variables|Default|GetPlayer)))
        (Variables|/Game/Blueprints/PlayerCharacter_BP.PlayerCharacter_BP_C|SetSMGAmmo (Variables|Default|GetPlayer) (Variables|/Game/Blueprints/PlayerCharacter_BP.PlayerCharacter_BP_C|GetMaxSMGAmmo (Variables|Default|GetPlayer)))))
    (:NewEnumerator3
      (Variables|/Game/Blueprints/PlayerCharacter_BP.PlayerCharacter_BP_C|SetShotgunAmmo (Variables|Default|GetPlayer) (+ (Variables|/Game/Blueprints/PlayerCharacter_BP.PlayerCharacter_BP_C|GetShotgunAmmo (Variables|Default|GetPlayer)) _ammo_2 (Variables|/Game/Blueprints/PlayerCharacter_BP.PlayerCharacter_BP_C|GetPendingShotgunAmmo (Variables|Default|GetPlayer))))
      (Variables|/Game/Blueprints/PlayerCharacter_BP.PlayerCharacter_BP_C|SetPendingShotgunAmmo (Variables|Default|GetPlayer) (- (Variables|/Game/Blueprints/PlayerCharacter_BP.PlayerCharacter_BP_C|GetPendingShotgunAmmo (Variables|Default|GetPlayer)) _ammo))
      (if (> (Variables|/Game/Blueprints/PlayerCharacter_BP.PlayerCharacter_BP_C|GetShotgunAmmo (Variables|Default|GetPlayer)) (Variables|/Game/Blueprints/PlayerCharacter_BP.PlayerCharacter_BP_C|GetMaxShotgunAmmo (Variables|Default|GetPlayer)))
        (Variables|/Game/Blueprints/PlayerCharacter_BP.PlayerCharacter_BP_C|SetShotgunAmmo (Variables|Default|GetPlayer) (Variables|/Game/Blueprints/PlayerCharacter_BP.PlayerCharacter_BP_C|GetMaxShotgunAmmo (Variables|Default|GetPlayer)))))
    (:NewEnumerator4
      (Variables|/Game/Blueprints/PlayerCharacter_BP.PlayerCharacter_BP_C|SetSniperRifleAmmo (Variables|Default|GetPlayer) (+ (Variables|/Game/Blueprints/PlayerCharacter_BP.PlayerCharacter_BP_C|GetSniperRifleAmmo (Variables|Default|GetPlayer)) _ammo_2 (Variables|/Game/Blueprints/PlayerCharacter_BP.PlayerCharacter_BP_C|GetPendingSniperRifleAmmo (Variables|Default|GetPlayer))))
      (Variables|/Game/Blueprints/PlayerCharacter_BP.PlayerCharacter_BP_C|SetPendingSniperRifleAmmo (Variables|Default|GetPlayer) (- (Variables|/Game/Blueprints/PlayerCharacter_BP.PlayerCharacter_BP_C|GetPendingSniperRifleAmmo (Variables|Default|GetPlayer)) _ammo))
      (if (> (Variables|/Game/Blueprints/PlayerCharacter_BP.PlayerCharacter_BP_C|GetSniperRifleAmmo (Variables|Default|GetPlayer)) (Variables|/Game/Blueprints/PlayerCharacter_BP.PlayerCharacter_BP_C|GetMaxSniperRifleAmmo (Variables|Default|GetPlayer)))
        (Variables|/Game/Blueprints/PlayerCharacter_BP.PlayerCharacter_BP_C|SetSniperRifleAmmo (Variables|Default|GetPlayer) (Variables|/Game/Blueprints/PlayerCharacter_BP.PlayerCharacter_BP_C|GetMaxSniperRifleAmmo (Variables|Default|GetPlayer)))))
    (:NewEnumerator5
      (Variables|/Game/Blueprints/PlayerCharacter_BP.PlayerCharacter_BP_C|SetRocketLauncherAmmo (Variables|Default|GetPlayer) (+ (Variables|/Game/Blueprints/PlayerCharacter_BP.PlayerCharacter_BP_C|GetRocketLauncherAmmo (Variables|Default|GetPlayer)) _ammo_2 (Variables|/Game/Blueprints/PlayerCharacter_BP.PlayerCharacter_BP_C|GetPendingRocketLauncherAmmo (Variables|Default|GetPlayer))))
      (Variables|/Game/Blueprints/PlayerCharacter_BP.PlayerCharacter_BP_C|SetPendingRocketLauncherAmmo (Variables|Default|GetPlayer) (- (Variables|/Game/Blueprints/PlayerCharacter_BP.PlayerCharacter_BP_C|GetPendingRocketLauncherAmmo (Variables|Default|GetPlayer)) _ammo))
      (if (> (Variables|/Game/Blueprints/PlayerCharacter_BP.PlayerCharacter_BP_C|GetRocketLauncherAmmo (Variables|Default|GetPlayer)) (Variables|/Game/Blueprints/PlayerCharacter_BP.PlayerCharacter_BP_C|GetMaxRocketLauncherAmmo (Variables|Default|GetPlayer)))
        (Variables|/Game/Blueprints/PlayerCharacter_BP.PlayerCharacter_BP_C|SetRocketLauncherAmmo (Variables|Default|GetPlayer) (Variables|/Game/Blueprints/PlayerCharacter_BP.PlayerCharacter_BP_C|GetMaxRocketLauncherAmmo (Variables|Default|GetPlayer)))))))

(event EventStartPending
  (bind _ammo (Variables|Default|GetAmmo))
  (bind _player (Variables|Default|GetPlayer))
  (switch Utilities|FlowControl|Switch|SwitchonWeaponTypes (Variables|Default|GetAmmoType)
    (:NewEnumerator0
      (Variables|/Game/Blueprints/PlayerCharacter_BP.PlayerCharacter_BP_C|SetPendingPistolAmmo _player (+ (Variables|/Game/Blueprints/PlayerCharacter_BP.PlayerCharacter_BP_C|GetPendingPistolAmmo _player) _ammo)))
    (:NewEnumerator1
      (Variables|/Game/Blueprints/PlayerCharacter_BP.PlayerCharacter_BP_C|SetPendingAssaultRifleAmmo _player (+ (Variables|/Game/Blueprints/PlayerCharacter_BP.PlayerCharacter_BP_C|GetPendingAssaultRifleAmmo _player) _ammo)))
    (:NewEnumerator2
      (Variables|/Game/Blueprints/PlayerCharacter_BP.PlayerCharacter_BP_C|SetPendingSMGAmmo _player (+ (Variables|/Game/Blueprints/PlayerCharacter_BP.PlayerCharacter_BP_C|GetPendingSMGAmmo _player) _ammo)))
    (:NewEnumerator3
      (Variables|/Game/Blueprints/PlayerCharacter_BP.PlayerCharacter_BP_C|SetPendingShotgunAmmo _player (+ (Variables|/Game/Blueprints/PlayerCharacter_BP.PlayerCharacter_BP_C|GetPendingShotgunAmmo _player) _ammo)))
    (:NewEnumerator4
      (Variables|/Game/Blueprints/PlayerCharacter_BP.PlayerCharacter_BP_C|SetPendingSniperRifleAmmo _player (+ (Variables|/Game/Blueprints/PlayerCharacter_BP.PlayerCharacter_BP_C|GetPendingSniperRifleAmmo _player) _ammo)))
    (:NewEnumerator5
      (Variables|/Game/Blueprints/PlayerCharacter_BP.PlayerCharacter_BP_C|SetPendingRocketLauncherAmmo _player (+ (Variables|/Game/Blueprints/PlayerCharacter_BP.PlayerCharacter_BP_C|GetPendingRocketLauncherAmmo _player) _ammo)))))

(fn ConstructionScript
  (|CallParentFunction))